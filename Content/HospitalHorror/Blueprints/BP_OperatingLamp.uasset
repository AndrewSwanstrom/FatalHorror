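; BP_OperatingLamp is a poseable operating-room lamp that can be on, off or flickering.
; The Construction Script toggles base visibility, rotates five parts from per-joint variables, and sets emissive and light intensities from LampOnoff.
; When lit and flickering, Tick plays a timeline whose track scales the head's emissive material, rect light and point light together.
; A TimerUpdate flag triggers a one-off jump to a random timeline time, randomizing the flicker phase.
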(event `self.ReceiveTick`
  (params (DeltaSeconds :type "Float (single-precision)"))
  (if (`self.Timer update`)
    (set `self.Timer update` false)
    (set `self.Timer` (`KismetMathLibrary.RandomFloatInRange` 0.0 12.0))
    (bind (_direction _newtrack_2) (`Timeline|Timeline_0` :`NewTime` (`self.Timer`) :!via `SetNewTime` :!label _label)
      (:`Update`
        (`MeshComponent.SetScalarParameterValueOnMaterials` (`self.OperatingLampPart01_6`) "Emissive Str" (* _newtrack_2 100.0))
        (`LightComponent.SetIntensity` (`self.RectLight`) (* _newtrack_2 20.0))
        (`LightComponent.SetIntensity` (`self.PointLight`) (* _newtrack_2 2.0))))
    (elif (`self.lamp on/off`)
      (if (`self.flickering lamp`)
        (goto _label)))))

(fn `UserConstructionScript`
  (`SceneComponent.SetVisibility` (`self.OperatingLampPart01_1`) (`self.Base Visivle on/off`) false)
  ;[1 1 1] Rotators
  (`SceneComponent.K2_SetRelativeRotation` (`self.OperatingLampPart01_2`) (`KismetMathLibrary.MakeRotator` 0.0 0.0 (`self.Part1_Rotator`)) false false)
  (`SceneComponent.K2_SetRelativeRotation` (`self.OperatingLampPart01_3`) (`KismetMathLibrary.MakeRotator` (`self.Part2_Rotator`)) false false)
  (`SceneComponent.K2_SetRelativeRotation` (`self.OperatingLampPart01_4`) (`KismetMathLibrary.MakeRotator` 0.0 0.0 (`self.Part3_Rotator`)) false false)
  (`SceneComponent.K2_SetRelativeRotation` (`self.OperatingLampPart01_5`) (`KismetMathLibrary.MakeRotator` 0.0 (`self.Part4_Rotator`)) false false)
  (`SceneComponent.K2_SetRelativeRotation` (`self.OperatingLampPart01_6`) (`KismetMathLibrary.MakeRotator` (`self.Part5_Rotator`)) false false)
  (if (`self.lamp on/off`)
    (`MeshComponent.SetScalarParameterValueOnMaterials` (`self.OperatingLampPart01_6`) "Emissive Str" 100.0)
    (`LightComponent.SetIntensity` (`self.RectLight`) 20.0)
    (`LightComponent.SetIntensity` (`self.PointLight`) 2.0)
    (else
      (`MeshComponent.SetScalarParameterValueOnMaterials` (`self.OperatingLampPart01_6`) "Emissive Str" 0.0)
      (`LightComponent.SetIntensity` (`self.RectLight`) 0.0)
      (`LightComponent.SetIntensity` (`self.PointLight`) 0.0))))