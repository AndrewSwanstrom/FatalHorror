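; BP_Lamp01 is a lamp actor whose rect light and mesh emissive glow vary together over time.
; The construction script applies the configurable color, emissive strength and light intensity to the Lamp01 materials and RectLight.
; A timeline track scales both strengths, with Tick calling Play repeatedly after a one-time jump to a random start time when TimerUpdate is set, staggering separate lamps.
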(event `self.ReceiveTick`
  (params (DeltaSeconds :type "Float (single-precision)"))
  (if (`self.Timer update`)
    (set `self.Timer update` false)
    (set `self.Timer` (`KismetMathLibrary.RandomFloatInRange` 0.0 12.0))
    (bind (_direction _newtrack_2) (`Timeline|Timeline_0` :`NewTime` (`self.Timer`) :!via `SetNewTime` :!label _label)
      (:`Update`
        (`MeshComponent.SetScalarParameterValueOnMaterials` (`self.Lamp01`) "Emissive Str" (* _newtrack_2 (`self.Emissive str`)))
        (`LightComponent.SetIntensity` (`self.RectLight`) (* _newtrack_2 (`self.Light intensity`)))))
    (else
      (goto _label))))

(fn `UserConstructionScript`
  (bind _rectlight (`self.RectLight`))
  (bind _lamp01 (`self.Lamp01`))
  (bind _light_color (`self.Light color`))
  (`MeshComponent.SetVectorParameterValueOnMaterials` _lamp01 "emissive color" (`KismetMathLibrary.Conv_LinearColorToVector` (`KismetMathLibrary.Conv_ColorToLinearColor` _light_color)))
  (`LightComponent.SetLightColor` _rectlight (`KismetMathLibrary.Conv_ColorToLinearColor` _light_color) true)
  (`MeshComponent.SetScalarParameterValueOnMaterials` _lamp01 "Emissive Str" (`self.Emissive str`))
  (`LightComponent.SetIntensity` _rectlight (`self.Light intensity`)))