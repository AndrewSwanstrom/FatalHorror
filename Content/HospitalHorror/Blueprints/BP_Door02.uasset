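; Automatic double sliding door for the hospital horror game that opens when something overlaps its Box trigger and closes when the overlap ends.
; Begin and end overlap set AutoOpen or AutoClose flags, which Tick reads to step DoorPosition between closed and a fixed open limit.
; The two door meshes slide apart along local Y in mirrored offsets, moving a fixed amount per frame without delta time, closing slightly faster than opening.
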(event `self.Box.OnComponentBeginOverlap`
  (params (OverlappedComponent :type "PrimitiveComponent Object Reference") (OtherActor :type "Actor Object Reference") (OtherComp :type "PrimitiveComponent Object Reference") (OtherBodyIndex :type Integer) (bFromSweep :type Boolean) (SweepResult :type "HitResult Structure (by ref)"))
  ;[1 1 1] AutoOpenAndColseDoor
  (set `self.Auto Close` false)
  (set `self.Auto Open` true))

(event `self.Box.OnComponentEndOverlap`
  (params (OverlappedComponent :type "PrimitiveComponent Object Reference") (OtherActor :type "Actor Object Reference") (OtherComp :type "PrimitiveComponent Object Reference") (OtherBodyIndex :type Integer))
  ;[1 1 1] AutoOpenAndColseDoor
  (set `self.Auto Close` true)
  (set `self.Auto Open` false))

(event `self.ReceiveTick`
  (params (DeltaSeconds :type "Float (single-precision)"))
  (bind _door_position (`self.Door Position`))
  (bind _door_position_2 (`self.Door Position`))
  (bind _door_position_3 (`self.Door Position`))
  ;[1 1 1] AutoOpenAndColseDoor
  (if (`self.Auto Open`)
    (`/Engine/EditorBlueprintResources/StandardMacros.CompareFloat` _door_position_3 80.0
      (:`>`
        (set `self.Door Position` 80.0 :!label _label)
        (set `self.Auto Open` false))
      (:`==`
        (goto _label))
      (:`<`
        (set `self.Door Position` (+ _door_position_3 1.6))
        (`SceneComponent.K2_SetRelativeLocation` (`self.Door01_7`) (+ (`KismetMathLibrary.MakeVector` 0.0 _door_position) (0.0 83.356133 0.0)) false false :!label _label_2)
        (`SceneComponent.K2_SetRelativeLocation` (`self.Door01_8`) (+ (`KismetMathLibrary.MakeVector` 0.0 (* _door_position -1.0)) (0.0 -83.356133 0.0)) false false)))
    (elif (`self.Auto Close`)
      (`/Engine/EditorBlueprintResources/StandardMacros.CompareFloat` _door_position_2
        (:`>`
          (set `self.Door Position` (- _door_position_2 2.0))
          (goto _label_2))
        (:`==`
          _)
        (:`<`
          _))
      (set `self.Door Position` 0.0)
      (set `self.Auto Close` false))))

(fn `UserConstructionScript`)